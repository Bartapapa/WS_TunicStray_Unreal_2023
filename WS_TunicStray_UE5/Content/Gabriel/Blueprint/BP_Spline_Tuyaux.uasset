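; Pipe spline actor (Tuyaux) that builds a run of deformed mesh segments along its spline in the Construction Script.
; Section length derives from the actor's X scale, and only whole sections are placed, dropping any remainder.
; Each segment takes its endpoints and tangents from the spline, with tangents clamped to section length to limit distortion.
; The CollisionsOn flag selects between two spline mesh component variants; there is no runtime logic.
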(fn `UserConstructionScript`
  (bind _returnvalue_x (`KismetMathLibrary.BreakVector` (`self.GetActorScale3D`)))
  (bind _spline (`self.Spline`))
  (bind _spline_2 (`self.Spline`))
  (set `self.Taillle Section` (* _returnvalue_x 100.0))
  (for _index (range (`KismetMathLibrary.FTrunc` (/ (`SplineComponent.GetSplineLength` (`self.Spline`)) (`self.Taillle Section`))))
    (if (`self.CollisionsOn`)
      (bind _returnvalue (`AddComponent|NODE_AddSplineMeshComponent-1`))
      (else
        (bind _returnvalue_2 (`AddComponent|NODE_AddSplineMeshComponent-2`))))
    (`SplineMeshComponent.SetForwardAxis` _returnvalue "X" true)
    (`PrimitiveComponent.SetCollisionEnabled` _returnvalue "NoCollision")
    (bind _returnvalue_3 (* _index (`self.Taillle Section`)))
    (bind _returnvalue_4 (* (+ _index 1) (`self.Taillle Section`)))
    (`SplineMeshComponent.SetStartAndEnd` _returnvalue (`SplineComponent.GetLocationAtDistanceAlongSpline` _spline _returnvalue_3 "Local") (`KismetMathLibrary.ClampVectorSize` (`SplineComponent.GetTangentAtDistanceAlongSpline` _spline _returnvalue_3 "Local") 0.0 (`self.Taillle Section`)) (`SplineComponent.GetLocationAtDistanceAlongSpline` _spline_2 _returnvalue_4 "Local") (`KismetMathLibrary.ClampVectorSize` (`SplineComponent.GetTangentAtDistanceAlongSpline` _spline_2 _returnvalue_4 "Local") 0.0 (`self.Taillle Section`)) true)
    (`SplineMeshComponent.SetStartAndEnd` _returnvalue_2 (`SplineComponent.GetLocationAtDistanceAlongSpline` _spline _returnvalue_3 "Local") (`KismetMathLibrary.ClampVectorSize` (`SplineComponent.GetTangentAtDistanceAlongSpline` _spline _returnvalue_3 "Local") 0.0 (`self.Taillle Section`)) (`SplineComponent.GetLocationAtDistanceAlongSpline` _spline_2 _returnvalue_4 "Local") (`KismetMathLibrary.ClampVectorSize` (`SplineComponent.GetTangentAtDistanceAlongSpline` _spline_2 _returnvalue_4 "Local") 0.0 (`self.Taillle Section`)) true)))